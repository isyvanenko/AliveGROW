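; BP_ExtraTime5s is a single-use pickup that adds extra time to the game timer.
; Any Sphere overlap passes TimeToAdd to the BP_Timer found in the level, plays pickup audio and a particle effect, then destroys the actor.
; A new W_ExtraTim widget notifies the player of the added time.
; Hide-and-respawn logic using a delay and collision toggle remains in the graph but is disconnected.
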(event `self.Sphere.OnComponentBeginOverlap`
  (params (OverlappedComponent :type "PrimitiveComponent Object Reference") (OtherActor :type "Actor Object Reference") (OtherComp :type "PrimitiveComponent Object Reference") (OtherBodyIndex :type Integer) (bFromSweep :type Boolean) (SweepResult :type "HitResult Structure (by ref)"))
  (`self.AddTime` (`self.TimeToAdd`))
  (`self.VisualRepExtraTime` (`self.PickUpSoundProject_Cue`) "/Game/FX_PickingUpExtraTime.FX_PickingUpExtraTime")
  (`self.UIupdate`)
  (`self.K2_DestroyActor`))

(fn `AddTime`
  (params (timeToAdd :type "Float (double-precision)"))
  (bind _returnvalue (`GameplayStatics.GetActorOfClass` "/Game/MyBlueprints/BP_Timer.BP_Timer_C"))
  (set `self.TimerBP` _returnvalue)
  (`/Game/MyBlueprints/BP_Timer.AddTime` (`self.TimerBP`) timeToAdd)
  (return))

(fn `Enab/DisableExtraTime`
  (params (NewType :type "ECollisionEnabled Enum" :default "NoCollision") (bNewHidden :type Boolean))
  (`PrimitiveComponent.SetCollisionEnabled` (`self.Sphere`) NewType)
  (`self.SetActorHiddenInGame` bNewHidden))

(fn `UIupdate`
  (bind _returnvalue (`|CreateWidget` "/Game/MyBlueprints/W_ExtraTim.W_ExtraTim_C"))
  (`UserWidget.AddToViewport` _returnvalue 0)
  (`/Game/MyBlueprints/W_ExtraTim.notifyplayerExtraTime` _returnvalue))

(fn `UserConstructionScript`)

(fn `VisualRepExtraTime`
  (params (PickUpAudio :type "AudioComponent Object Reference") (PickUpParticle :type "NiagaraSystem Object Reference"))
  (`AudioComponent.Play` PickUpAudio 0.0)
  (`NiagaraFunctionLibrary.SpawnSystemAtLocation` PickUpParticle (`self.K2_GetActorLocation`)))
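; BP_WateringCan is a tool actor that the first-person character picks up and uses to water plants.
; Overlapping its box passes the can to the character's PickUpTool.
; UseWateringCan tells an already watered plant it is done; otherwise it decrements the plant's Progress, plays audio and has the plant run its completion and progress checks.
; The validity check on the target plant runs only after its Watered flag is read.
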(event `self.Box.OnComponentBeginOverlap`
  (params (OverlappedComponent :type "PrimitiveComponent Object Reference") (OtherActor :type "Actor Object Reference") (OtherComp :type "PrimitiveComponent Object Reference") (OtherBodyIndex :type Integer) (bFromSweep :type Boolean) (SweepResult :type "HitResult Structure (by ref)"))
  (bind _asbp_first_person_character (cast `/Game/FirstPerson/Blueprints/BP_FirstPersonCharacter` OtherActor))
  (`/Game/FirstPerson/Blueprints/BP_FirstPersonCharacter.PickUpTool` _asbp_first_person_character self))

(fn `UserConstructionScript`
  (`parent.UserConstructionScript`))

(fn `UseWateringCan`
  (params (TargetPlant :type "/Game/MyBlueprints/BP_Plant Object Reference"))
  (if (`/Game/MyBlueprints/BP_Plant.Watered?` TargetPlant)
    (`/Game/MyBlueprints/BP_Plant.AlreadyBeenDone` TargetPlant false false true)
    (else
      (`/Engine/EditorBlueprintResources/StandardMacros.IsValid` TargetPlant
        (:`Is Valid`
          (bind _result (`/Engine/EditorBlueprintResources/StandardMacros.DecrementInt` (`/Game/MyBlueprints/BP_Plant.Progress` TargetPlant))
            (:`  `
              (set `/Game/MyBlueprints/BP_Plant.Progress` _result TargetPlant)
              (`AudioComponent.Play` (`self.Audio`) 0.0)
              (`/Game/MyBlueprints/BP_Plant.CheckIfAllDone` TargetPlant true false false)
              (`/Game/MyBlueprints/BP_Plant.CheckProgress` TargetPlant))))))))
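; BP_CameraMoveMenu is a Blueprint that gives a camera, by its name one used for the menu, a continuous vertical bobbing motion.
; BeginPlay stores the Camera component's relative location as the origin.
; Each Tick offsets only the Z of that origin by a sine of game time, scaled by speed and amplitude variables, so the motion oscillates around the start point without drifting.
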(event `self.ReceiveBeginPlay`
  (set `self.OriginalPosition` (`SceneComponent.RelativeLocation` (`self.Camera`))))

(event `self.ReceiveTick`
  (params (DeltaSeconds :type "Float (single-precision)"))
  (`SceneComponent.K2_SetRelativeLocation` (`self.Camera`) (`KismetMathLibrary.MakeVector` (.x (`self.OriginalPosition`)) (.y (`self.OriginalPosition`)) (+ (.z (`self.OriginalPosition`)) (* (`KismetMathLibrary.Sin` (* (`KismetSystemLibrary.GetGameTimeInSeconds`) (`self.SpeedOfTheMovement`))) (`self.Amplitude`)))) false false))

(fn `UserConstructionScript`)
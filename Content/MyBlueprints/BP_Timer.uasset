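; BP_Timer is a game countdown timer that opens the L_GameOver level when its game-over check passes.
; Tick subtracts delta seconds from GameTime through DecreaseGameTime, then calls IsGameOver, whose graph shows a zero-or-below comparison but no connected output.
; AddTime and RemoveTime adjust GameTime by a given amount and print the new value as debug text.
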(event `self.ReceiveTick`
  (params (DeltaSeconds :type "Float (single-precision)"))
  (set `self.GameTime` (- (`self.GameTime`) DeltaSeconds))
  (if (<= (`self.GameTime`) 0.0)
    (`GameplayStatics.OpenLevel` "L_GameOver")))

(fn `AddTime`
  (params (timeToAdd :type "Float (double-precision)"))
  (bind _output_get (set `self.GameTime` (+ (`self.GameTime`) timeToAdd)))
  (`KismetSystemLibrary.PrintString` (`KismetStringLibrary.Concat_StrStr` (`KismetStringLibrary.Conv_DoubleToString` _output_get) " Time Added!") true true (struct :`R` 0.0979 :`G` 1.0 :`A` 1.0))
  (return))

(fn `RemoveTime`
  (params (timeToRemove :type "Float (double-precision)"))
  (bind _output_get (set `self.GameTime` (- (`self.GameTime`) timeToRemove)))
  (`KismetSystemLibrary.PrintString` (`KismetStringLibrary.Concat_StrStr` (`KismetStringLibrary.Conv_DoubleToString` _output_get) " Time Removed!") true true (struct :`R` 1.0 :`B` 0.004961 :`A` 1.0))
  (return))

(fn `UserConstructionScript`)